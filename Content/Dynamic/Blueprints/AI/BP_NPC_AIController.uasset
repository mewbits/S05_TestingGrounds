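; AI controller for guard NPCs that makes them aim at actors they perceive.
; On BeginPlay it starts the BB_PatrolData blackboard and BT_GuardBase behavior tree, then caches the controlled TP_Character.
; AI perception updates ignore actors whose first tag is "Enemy", while untagged actors still count.
; Sensing a target sets the FocusActor key and the character's Aiming flag; losing any accepted target clears both.
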(event `self.ReceiveBeginPlay`
  (bind _blackboardcomponent (`self.UseBlackboard` "/Game/Dynamic/Blueprints/AI/BB_PatrolData.BB_PatrolData"))
  (set `self.BlackboardRef` _blackboardcomponent)
  (`self.RunBehaviorTree` "/Game/Dynamic/Blueprints/AI/BT_GuardBase.BT_GuardBase")
  (bind _astp_character (cast `/Game/Dynamic/Blueprints/TP_Character` (`self.K2_GetPawn`)))
  (set `self.AICharacter` _astp_character))

(event `self.AIPerception.OnTargetPerceptionUpdated`
  (params (Actor :type "Actor Object Reference") (Stimulus :type "AIStimulus Structure"))
  (bind _aicharacter (`self.AICharacter`))
  (bind _tags (`Actor.Tags` Actor))
  (bind _blackboardref (`self.BlackboardRef`))
  (bind _aicharacter_2 (`self.AICharacter`))
  (if (`KismetArrayLibrary.Array_IsValidIndex` _tags)
    (if (!= (`|GetArrayItem` _tags) "Enemy")
      (if (`.bSuccessfullySensed` (break `AIStimulus` Stimulus)) :!label _label
        (`BlackboardComponent.SetValueAsObject` _blackboardref "FocusActor" Actor)
        (`/Engine/EditorBlueprintResources/StandardMacros.IsValid` _aicharacter_2
          (:`Is Valid`
            (set `/Game/Dynamic/Blueprints/TP_Character.Aiming` true _aicharacter_2)))
        (else
          (`BlackboardComponent.ClearValue` _blackboardref "FocusActor")
          (`/Engine/EditorBlueprintResources/StandardMacros.IsValid` _aicharacter
            (:`Is Valid`
              (set `/Game/Dynamic/Blueprints/TP_Character.Aiming` false _aicharacter))))))
    (else
      (goto _label))))

(fn `UserConstructionScript`)